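; BP_Enemy1 is an enemy that wanders around its spawn point and chases the player character on sight.
; Patrullar line-traces downward between random points within RadioDeMovimiento to find a ground destination, issues AI MoveTo, then repeats after a delay.
; PawnSensing sightings of a ThirdPersonCharacter issue a chase MoveTo and refresh a Retriggerable Delay, which calls Patrullar again once sightings stop.
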(event OnSeePawn(PawnSensing)
  (params (Pawn :type Pawn%20Object%20Reference))
  (bind _asthird_person_character (Utilities|Casting|CastToThirdPersonCharacter Pawn))
  (AI|AIMoveTo self "0, 0, 0" _asthird_person_character 1.2e+02 false
    (:then
      (Utilities|FlowControl|RetriggerableDelay 1.0)
      (CallFunction|Patrullar))))

(event Custom|Patrullar
  (bind _ubicacioninicial (Variables|Default|GetUbicacionInicial))
  (bind _radiodemovimiento (Variables|Default|GetradioDeMovimiento))
  (bind _radiodemovimiento_2 (Variables|Default|GetradioDeMovimiento))
  (bind _radiodemovimiento_3 (Variables|Default|GetradioDeMovimiento))
  (bind _radiodemovimiento_4 (Variables|Default|GetradioDeMovimiento))
  (bind _returnvalue (* _radiodemovimiento -1.0))
  (bind _returnvalue_2 (* _radiodemovimiento_4 -1.0))
  (bind _returnvalue_3 (Math|Random|RandomFloatinRange _returnvalue _radiodemovimiento_2))
  (bind _returnvalue_4 (Math|Random|RandomFloatinRange _returnvalue_2 _radiodemovimiento_3))
  (bind _returnvalue_5 (+ _returnvalue_4 (.x _ubicacioninicial)))
  (bind _returnvalue_6 (+ _returnvalue_3 (.y _ubicacioninicial)))
  (bind _outhit (Collision|LineTraceByChannel (Math|Vector|MakeVector _returnvalue_5 _returnvalue_6 2e+04) (Math|Vector|MakeVector _returnvalue_5 _returnvalue_6 -1e+04) "TraceTypeQuery1" true 0 "None" true "(R=1.000000,G=0.000000,B=0.000000,A=1.000000)" "(R=0.000000,G=1.000000,B=0.000000,A=1.000000)" 1e+03 :!label _label))
  (AI|AIMoveTo self (.ImpactPoint (Collision|BreakHitResult _outhit)) 0 5.0 false
    (:then
      (Utilities|FlowControl|Delay 5.0)
      (goto _label))))

(event EventBeginPlay
  (Variables|Default|SetUbicacionInicial (Transformation|GetActorLocation))
  (CallFunction|Patrullar))

(fn ConstructionScript)