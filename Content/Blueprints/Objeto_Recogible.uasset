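; Pickup actor that the player collects by holding the interaction input while inside its box, which destroys the actor.
; Overlap by the ThirdPersonCharacter enables input, shows a Hold_E_To_Pick_Up widget and opens a gate; leaving reverses this.
; A press starts a retriggerable delay of MaxHoldTime that destroys the actor if still held.
; A parallel timer, polled recursively, feeds held time to the widget until release resets it.
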(event OnComponentBeginOverlap(Box)
  (params (OverlappedComponent :type Primitive%20Component%20Object%20Reference) (OtherActor :type Actor%20Object%20Reference) (OtherComp :type Primitive%20Component%20Object%20Reference) (OtherBodyIndex :type Integer) (bFromSweep :type Boolean) (SweepResult :type Hit%20Result%20Structure%20%28by%20ref%29))
  ;[1 1 1] interaccion con objeto
  (Utilities|Casting|CastToThirdPersonCharacter OtherActor)
  (Input|EnableInput (Game|GetPlayerController 0))
  (bind _returnvalue (UserInterface|CreateWidget "/Game/Menus/Hold_E_To_Pick_Up.Hold_E_To_Pick_Up_C"))
  (bind _output_get (Variables|Default|SetNewVar_0 _returnvalue))
  (UserInterface|Viewport|AddtoViewport _output_get 0)
  (Variables|/Game/Menus/Hold_E_To_Pick_Up.Hold_E_To_Pick_Up_C|SetMaxTimeHeld _output_get (Variables|Default|GetMaxHoldTime))
  (Utilities|FlowControl|Gate true) ; enters at Open
)

(event OnComponentEndOverlap(Box)
  (params (OverlappedComponent :type Primitive%20Component%20Object%20Reference) (OtherActor :type Actor%20Object%20Reference) (OtherComp :type Primitive%20Component%20Object%20Reference) (OtherBodyIndex :type Integer))
  ;[1 1 1] interaccion con objeto
  (Utilities|Casting|CastToThirdPersonCharacter OtherActor)
  (Input|DisableInput (Game|GetPlayerController 0))
  (Widget|RemovefromParent (stale OnComponentBeginOverlap(Box) _returnvalue))
  (Utilities|FlowControl|Gate true) ; enters at Close
)

(event Custom|Timer
  ;[1 1 1] controlar tiempo de uso
  (bind _returnvalue (Utilities|Time|SetTimerbyEvent (delegate Custom|Timer) (Variables|Default|GetMaxHoldTime))))

(event Custom|Stop%20Timer
  ;[1 1 1] controlar tiempo de uso
  (Utilities|Time|PauseTimerbyHandle (stale Custom|Timer _returnvalue)))

(event Custom|Update%20timer
  (bind _newvar_0 (Variables|Default|GetNewVar_0))
  ;[1 1 1] controlar tiempo de uso
  (if (Variables|Default|GetisHeld)
    (Variables|/Game/Menus/Hold_E_To_Pick_Up.Hold_E_To_Pick_Up_C|SetTimeHeld _newvar_0 (Class|KismetSystemLibrary|GetTimerElapsedTimeHandle (stale Custom|Timer _returnvalue)))
    (Utilities|FlowControl|Delay 0.1)
    (CallFunction|UpdateTimer)
    (else
      (CallFunction|StopTimer)
      (Variables|/Game/Menus/Hold_E_To_Pick_Up.Hold_E_To_Pick_Up_C|SetTimeHeld _newvar_0 0.0))))

(event Input|ActionEvents|InputActioninteraction
  (params (Key :type Key%20Structure))
  ;[1 1 1] interaccion con objeto
  (:Pressed
    (Variables|Default|SetisHeld true)
    (Utilities|FlowControl|Gate true
      (:Exit
        (Utilities|FlowControl|Sequence
          (:then_0
            (Utilities|FlowControl|RetriggerableDelay (Variables|Default|GetMaxHoldTime))
            (if (Variables|Default|GetisHeld)
              (Actor|DestroyActor)))
          (:then_1
            (CallFunction|Timer)
            (CallFunction|UpdateTimer))))))
  (:Released
    (Variables|Default|SetisHeld false)))

(fn ConstructionScript)